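; BP_EndZone is a trigger zone that decides whether the player can finish the game on reaching it.
; When a ThirdPersonCharacter overlaps, it queries the game manager: zero doors opened shows game status, while three opened either changes game state if all lives are saved or shows a save-more prompt.
; One or two opened doors trigger nothing.
; Ending the Overlap component's overlap hides both messages.
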(event `self.ReceiveActorBeginOverlap`
  (params (OtherActor :type "Actor Object Reference"))
  (cast `/Game/ThirdPersonBP/Blueprints/ThirdPersonCharacter` OtherActor)
  (bind _my_game_manager (`/Game/_MyContent/Blueprints/BP_MyFunctionLibrary.Get My Game Manager`))
  (if (== (`/Game/_MyContent/Blueprints/BP_MyGameManager.DoorsOpened` _my_game_manager) 0)
    (`/Game/_MyContent/Blueprints/BP_MyGameManager.Show Game Status` _my_game_manager true)
    (elif (== (`/Game/_MyContent/Blueprints/BP_MyGameManager.DoorsOpened` _my_game_manager) 3)
      (if (== (`/Game/_MyContent/Blueprints/BP_MyGameManager.MaxSaveLives` _my_game_manager) (`/Game/_MyContent/Blueprints/BP_MyGameManager.LivesSaved` _my_game_manager))
        (`/Game/_MyContent/Blueprints/BP_MyGameManager.Set State` _my_game_manager "NewEnumerator1")
        (else
          (`/Game/_MyContent/Blueprints/BP_MyGameManager.Show Save More` _my_game_manager true))))))

(event `self.Overlap.OnComponentEndOverlap`
  (params (OverlappedComponent :type "PrimitiveComponent Object Reference") (OtherActor :type "Actor Object Reference") (OtherComp :type "PrimitiveComponent Object Reference") (OtherBodyIndex :type Integer))
  (cast `/Game/ThirdPersonBP/Blueprints/ThirdPersonCharacter` OtherActor)
  (bind _my_game_manager (`/Game/_MyContent/Blueprints/BP_MyFunctionLibrary.Get My Game Manager`))
  (`/Game/_MyContent/Blueprints/BP_MyGameManager.Show Game Status` _my_game_manager false)
  (`/Game/_MyContent/Blueprints/BP_MyGameManager.Show Save More` _my_game_manager false))

(fn `UserConstructionScript`)