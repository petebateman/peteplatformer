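; BP_Key is a collectible key pickup with a KeyType of None, Blue, Green or Gold.
; The construction script sets the key mesh's material from that type.
; When a ThirdPersonCharacter enters the overlap component, the key adds its type to the character's OwnedKeys, destroys itself and plays a coin collect sound at the world origin.
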(event `self.Overlap.OnComponentBeginOverlap`
  (params (OverlappedComponent :type "PrimitiveComponent Object Reference") (OtherActor :type "Actor Object Reference") (OtherComp :type "PrimitiveComponent Object Reference") (OtherBodyIndex :type Integer) (bFromSweep :type Boolean) (SweepResult :type "HitResult Structure (by ref)"))
  (bind _asthird_person_character (cast `/Game/ThirdPersonBP/Blueprints/ThirdPersonCharacter` OtherActor))
  (`KismetArrayLibrary.Array_Add` (`/Game/ThirdPersonBP/Blueprints/ThirdPersonCharacter.OwnedKeys` _asthird_person_character) (`self.KeyType`))
  (`self.K2_DestroyActor`)
  (`GameplayStatics.PlaySoundAtLocation` "/Game/Audio/SoundEffects/Coin-collect-sound-effect.Coin-collect-sound-effect" (0.0 0.0 0.0) (struct) 1.0 1.0 0.0 null null null))

(fn `UserConstructionScript`
  (`PrimitiveComponent.SetMaterial` (`self.Key`) 0 (select `/Game/_MyContent/Blueprints/E_KeyType` (`self.KeyType`) :`NewEnumerator0` "/Game/_MyContent/Materials/M_Key.M_Key" :`NewEnumerator1` "/Game/_MyContent/Materials/M_BlueKey.M_BlueKey" :`NewEnumerator2` "/Game/_MyContent/Materials/M_GreenKey.M_GreenKey" :`NewEnumerator3` "/Game/_MyContent/Materials/M_GoldKey.M_GoldKey" :!type "MaterialInterface Object Reference")))