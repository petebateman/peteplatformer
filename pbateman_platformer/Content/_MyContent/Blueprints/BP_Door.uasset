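; BP_Door is a locked door that opens when a ThirdPersonCharacter carrying its RequiredKeyType enters the Overlap component.
; Each matching entry in OwnedKeys removes index 0 (not necessarily the match), sets IsOpen, increments the game manager's DoorsOpened and plays a sound at world origin.
; The OpenDoor timeline then drives the Arrow component's relative yaw to swing the door.
; The loop has no break or IsOpen check.
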(event `self.Overlap.OnComponentBeginOverlap`
  (params (OverlappedComponent :type "PrimitiveComponent Object Reference") (OtherActor :type "Actor Object Reference") (OtherComp :type "PrimitiveComponent Object Reference") (OtherBodyIndex :type Integer) (bFromSweep :type Boolean) (SweepResult :type "HitResult Structure (by ref)"))
  (bind _asthird_person_character (cast `/Game/ThirdPersonBP/Blueprints/ThirdPersonCharacter` OtherActor))
  (bind _ownedkeys (`/Game/ThirdPersonBP/Blueprints/ThirdPersonCharacter.OwnedKeys` _asthird_person_character))
  (for _array_element _ownedkeys
    (if (`|EnumEquality` _array_element (`self.RequiredKeyType`))
      (`KismetArrayLibrary.Array_Remove` _ownedkeys)
      (set `self.IsOpen?` true)
      (bind _my_game_manager (`/Game/_MyContent/Blueprints/BP_MyFunctionLibrary.Get My Game Manager`))
      (set `/Game/_MyContent/Blueprints/BP_MyGameManager.DoorsOpened` (+ (`/Game/_MyContent/Blueprints/BP_MyGameManager.DoorsOpened` _my_game_manager) 1) _my_game_manager)
      (`GameplayStatics.PlaySoundAtLocation` "/Game/Audio/SoundEffects/Wooden-door-opening-sound-effect.Wooden-door-opening-sound-effect" (0.0 0.0 0.0) (struct) 1.0 1.0 0.0 null null null)
      (bind (_direction _open_door) (`Timeline|Open Door`)
        (:`Update`
          (`SceneComponent.K2_SetRelativeRotation` (`self.Arrow`) (`KismetMathLibrary.MakeRotator` 0.0 0.0 (.z (`KismetMathLibrary.MakeVector` 0.0 0.0 _open_door))) false false))))))

(fn `UserConstructionScript`)